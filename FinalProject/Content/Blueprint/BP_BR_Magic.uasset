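; BP_BR_Magic is a short-lived Bringer spell attack that damages BP_MainPlayer, then destroys itself after chained delays from BeginPlay.
; Tick plays the spell flipbook and sound once after a short delay, and separately calls HitCheck through a repeating Delay.
; HitCheck applies BRMagicDMG to players overlapping HitBox.
; Its CheckHit guard is set back to false after damage, so it does not block repeat hits.
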(event `self.ReceiveBeginPlay`
  (`KismetSystemLibrary.Delay` 0.5)
  (`KismetSystemLibrary.Delay` 1.0)
  (`self.K2_DestroyActor`))

(event `self.ReceiveTick`
  (params (DeltaSeconds :type "Float (single-precision)"))
  (`|ExecutionSequence`
    (:`then_0`
      (`/Engine/EditorBlueprintResources/StandardMacros.DoOnce` false
        (:`Completed`
          (`KismetSystemLibrary.Delay` 0.5)
          (`PaperFlipbookComponent.SetFlipbook` (`self.Sprite`) "/Game/Asset/Bringer-Of-Death/Individual_Sprite/Spell/Bringer_Spell.Bringer_Spell")
          (`GameplayStatics.PlaySound2D` "/Game/Asset/Sound/BR_Magic.BR_Magic" 1.5 1.0 0.0 "/Game/Blueprint/BP_SoundConcurrency.BP_SoundConcurrency" null))))
    (:`then_1`
      (`KismetSystemLibrary.Delay` 0.5)
      (`self.HitCheck`))))

(fn `HitCheck`
  (for _array_element (`PrimitiveComponent.GetOverlappingActors` (`self.HitBox`) "/Game/Blueprint/BP_MainPlayer.BP_MainPlayer_C")
    (if (!= _array_element self)
      (if (not (`self.CheckHit`))
        (`GameplayStatics.ApplyDamage` _array_element (`self.BR_MagicDMG`))
        (set `self.CheckHit` false)))))

(fn `UserConstructionScript`)