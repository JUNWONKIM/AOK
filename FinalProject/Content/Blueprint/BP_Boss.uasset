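; Flipbook-animated 2D boss that casts random spells, takes damage and, on death, updates score and spawn state in BP_PlayerData.
; Tick fires EnemyAtk once the enemy count is zero and the boss is free, picking an animation and one of four attack actors spawned near player or boss.
; Sprite finish returns to idle and re-arms attacks and their frame-timed sound.
; AnyDamage drives hit and death animations and raises the player's combo.
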(event `self.ReceiveBeginPlay`
  (`|ExecutionSequence`
    (:`then_0`
      (`PaperFlipbookComponent.SetFlipbook` (`self.Sprite`) "/Game/Asset/Boss/Boss_Spawn.Boss_Spawn")
      (`PaperFlipbookComponent.SetLooping` (`self.Sprite`) false))
    (:`then_3`
      (bind _asbp_player_data (cast `/Game/Blueprint/BP_PlayerData` (`GameplayStatics.GetPlayerState` 0)))
      (bind _output_get (set `self.As BP Player Data` _asbp_player_data))
      (set `/Game/Blueprint/BP_PlayerData.PD_SetEnemyCount` 7 _output_get))
    (:`then_7`
      (bind _asbp_main_player (cast `/Game/Blueprint/BP_MainPlayer` (`GameplayStatics.GetPlayerCharacter` 0)))
      (set `self.As BP Main Player` _asbp_main_player))))

(event `Spawn Magic`
  ;[1 1 1] Boss Attack
  (if (`self.Boss_SetDarkAtk`)
    (if (`KismetMathLibrary.RandomBool`)
      (`|SpawnActorFromClass` "/Game/Blueprint/BP_Boss_Atk1.BP_Boss_Atk1_C" (`KismetMathLibrary.MakeTransform` (+ (`self.K2_GetActorLocation` (`self.As BP Main Player`)) (0.0 0.1 0.0))) "Undefined" "OverrideRootScale" null null)
      (else
        (`|SpawnActorFromClass` "/Game/Blueprint/BP_Boss_Atk4.BP_Boss_Atk4_C" (`KismetMathLibrary.MakeTransform` (+ (`self.K2_GetActorLocation`) (-30.0 0.1 0.0))) "Undefined" "OverrideRootScale" null null)))
    (elif (`KismetMathLibrary.RandomBool`)
      (`|SpawnActorFromClass` "/Game/Blueprint/BP_Boss_Atk2.BP_Boss_Atk2_C" (`KismetMathLibrary.MakeTransform` (+ (`self.K2_GetActorLocation` (`self.As BP Main Player`)) (0.0 0.1 0.0))) "Undefined" "OverrideRootScale" null null)
      (else
        (`|SpawnActorFromClass` "/Game/Blueprint/BP_Boss_Atk3.BP_Boss_Atk3_C" (`KismetMathLibrary.MakeTransform` (+ (`self.K2_GetActorLocation` (`self.As BP Main Player`)) (0.0 0.1 0.0))) "Undefined" "OverrideRootScale" null null)
        (`KismetSystemLibrary.Delay` 0.5)
        (`|SpawnActorFromClass` "/Game/Blueprint/BP_Boss_Atk3.BP_Boss_Atk3_C" (`KismetMathLibrary.MakeTransform` (+ (`self.K2_GetActorLocation` (`self.As BP Main Player`)) (0.0 0.1 0.0))) "Undefined" "OverrideRootScale" null null)))))

(event `Enemy Atk`
  (bind _sprite (`self.Sprite`))
  ;[1 0.7554 0.5051] Boss_Attack
  (if (== (`/Game/Blueprint/BP_PlayerData.PD_EnemyCount` (`self.As BP Player Data`)) 0)
    (if (`self.Boss_TakeHit`)
      _
      (elif (`self.Boss_Die`)
        _
        (elif (not (`/Game/Blueprint/BP_PlayerData.PD_IsEnemyAttack` (`self.As BP Player Data`)))
          (if (`KismetMathLibrary.RandomBool`)
            (`PaperFlipbookComponent.SetFlipbook` _sprite "/Game/Asset/Boss/Boss_Atk.Boss_Atk")
            (set `self.Boss_SetDarkAtk` true)
            (else
              (`PaperFlipbookComponent.SetFlipbook` _sprite "/Game/Asset/Boss/Boss_Atk2.Boss_Atk2")
              (set `self.Boss_SetDarkAtk` false)))
          (`self.Spawn Magic`)
          (set `/Game/Blueprint/BP_PlayerData.PD_CanBlockATK` true (`self.As BP Player Data`))
          (`PaperFlipbookComponent.SetLooping` (`self.Sprite`) false)
          (set `/Game/Blueprint/BP_PlayerData.PD_IsEnemyAttack` true (`self.As BP Player Data`)))))))

(event `self.Sprite.OnFinishedPlaying`
  ;[0.4018 0.6503 1] Boss_Idle
  (if (not (`self.Boss_Die`))
    (`PaperFlipbookComponent.SetFlipbook` (`self.Sprite`) "/Game/Asset/Boss/Boss_Idle.Boss_Idle")
    (`self.Looping`)
    (set `/Game/Blueprint/BP_PlayerData.PD_IsEnemyAttack` false (`self.As BP Player Data`))
    (set `self.Boss_TakeHit` false)
    (`self.ResetAttack`)))

(event `self.ReceiveTick`
  (params (DeltaSeconds :type "Float (single-precision)"))
  ;[1 0.9671 0.3297] Event Tick
  (`|ExecutionSequence`
    (:`then_2`
      (`self.Enemy Atk`))
    (:`then_4`
      (if (`/Game/Blueprint/BP_PlayerData.PD_IsEnemyAttack` (`self.As BP Player Data`))
        (if (== (`PaperFlipbookComponent.GetPlaybackPositionInFrames` (`self.Sprite`)) 7)
          (`/Engine/EditorBlueprintResources/StandardMacros.DoOnce` false :!label _label
            (:`Completed`
              (`GameplayStatics.PlaySound2D` "/Game/Asset/Sound/Boss_Atk.Boss_Atk" 1.0 1.0 0.0 "/Game/Blueprint/BP_SoundConcurrency.BP_SoundConcurrency" null))))))))

(event `ResetAttack`
  ;[1 0.9671 0.3297] Event Tick
  (goto _label :!via `Reset`))

(event `self.ReceiveAnyDamage`
  (params (Damage :type "Float (single-precision)") (DamageType :type "DamageType Object Reference") (InstigatedBy :type "Controller Object Reference") (DamageCauser :type "Actor Object Reference"))
  (bind _as_bp_player_data (`self.As BP Player Data`))
  (bind _boss_hp (`self.Boss_HP`))
  (bind _as_bp_player_data_2 (`self.As BP Player Data`))
  ;[0.4464 0.3844 1] Get Damage
  (set `self.Boss_HP` (- _boss_hp Damage))
  (if (<= _boss_hp 0.0)
    (set `self.Boss_Die` true)
    (`GameplayStatics.PlaySound2D` "/Game/Asset/Sound/Boss_Spawn.Boss_Spawn" 0.5 1.0 0.0 "/Game/Blueprint/BP_SoundConcurrency.BP_SoundConcurrency" null)
    (`PaperFlipbookComponent.SetFlipbook` (`self.Sprite`) "/Game/Asset/Boss/Boss_Die.Boss_Die")
    (`PaperFlipbookComponent.SetLooping` (`self.Sprite`) false)
    (`|ExecutionSequence`
      (:`then_0`
        (`KismetSystemLibrary.Delay` 1.0)
        (set `/Game/Blueprint/BP_PlayerData.PD_IsEnemySpawn` false (`self.As BP Player Data`))
        (set `/Game/Blueprint/BP_PlayerData.PD_BossCount` 5 (`self.As BP Player Data`))
        (set `/Game/Blueprint/BP_PlayerData.PD_Score` (+ (`/Game/Blueprint/BP_PlayerData.PD_Score` _as_bp_player_data_2) 10) _as_bp_player_data_2)
        (`self.K2_DestroyActor`))
      (:`then_1`
        (set `/Game/Blueprint/BP_PlayerData.PD_PlayerComboCount` (+ (`/Game/Blueprint/BP_PlayerData.PD_PlayerComboCount` _as_bp_player_data) 1) _as_bp_player_data :!label _label_2)))
    (else
      (set `self.Boss_TakeHit` true)
      (`PaperFlipbookComponent.SetFlipbook` (`self.Sprite`) "/Game/Asset/Boss/Boss_TakeHit.Boss_TakeHit")
      (`PaperFlipbookComponent.SetLooping` (`self.Sprite`) false)
      (goto _label_2))))

(fn `Looping`
  (`PaperFlipbookComponent.SetLooping` (`self.Sprite`) true)
  (if (not (`PaperFlipbookComponent.IsPlaying` (`self.Sprite`)))
    (`PaperFlipbookComponent.Play` (`self.Sprite`))))

(fn `UserConstructionScript`)