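; BP_Boss_Atk2 is a boss thunder attack that chains along +X as a short row of self-spawning strikes.
; After a brief delay, each strike spawns the next, using a counter in BP_PlayerData to cap and reset the chain, and destroys itself shortly after.
; Tick plays the thunder sound and delayed flipbook swap once, and repeatedly runs a delayed HitBox overlap check that damages BP_MainPlayer once per strike.
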(event `self.ReceiveBeginPlay`
  (bind _as_bp_player_data (`self.As BP Player Data`))
  (`|ExecutionSequence`
    (:`then_0`
      (bind _asbp_player_data (cast `/Game/Blueprint/BP_PlayerData` (`GameplayStatics.GetPlayerState` 0)))
      (set `self.As BP Player Data` _asbp_player_data))
    (:`then_1`
      (`KismetSystemLibrary.Delay` 0.5)
      (if (< (`/Game/Blueprint/BP_PlayerData.PD_Boss_Atk2NUM` (`self.As BP Player Data`)) 2)
        (`|SpawnActorFromClass` "BP_Boss_Atk2_C" (`KismetMathLibrary.MakeTransform` (+ (`self.K2_GetActorLocation`) (50.0 0.0 0.0))) "Undefined" "OverrideRootScale" null null)
        (set `/Game/Blueprint/BP_PlayerData.PD_Boss_Atk2NUM` (+ (`/Game/Blueprint/BP_PlayerData.PD_Boss_Atk2NUM` _as_bp_player_data) 1) _as_bp_player_data)
        (else
          (set `/Game/Blueprint/BP_PlayerData.PD_Boss_Atk2NUM` 0 (`self.As BP Player Data`)))))
    (:`then_3`
      (`KismetSystemLibrary.Delay` 1.0)
      (`self.K2_DestroyActor`))))

(event `self.ReceiveTick`
  (params (DeltaSeconds :type "Float (single-precision)"))
  (`|ExecutionSequence`
    (:`then_0`
      (`/Engine/EditorBlueprintResources/StandardMacros.DoOnce` false
        (:`Completed`
          (`GameplayStatics.PlaySound2D` "/Game/Asset/Sound/Boss_Thunder2.Boss_Thunder2" 1.0 1.0 0.0 "/Game/Blueprint/BP_SoundConcurrency.BP_SoundConcurrency" null)
          (`KismetSystemLibrary.Delay` 1.0)
          (`PaperFlipbookComponent.SetFlipbook` (`self.Sprite`) "/Game/Asset/Boss/BossEffect/Boss_Atk3.Boss_Atk3"))))
    (:`then_1`
      (`KismetSystemLibrary.Delay` 0.3)
      (`self.HitCheck`))))

(fn `HitCheck`
  (for _array_element (`PrimitiveComponent.GetOverlappingActors` (`self.HitBox`) "/Game/Blueprint/BP_MainPlayer.BP_MainPlayer_C")
    (if (!= _array_element self)
      (if (not (`self.CheckHit`))
        (`GameplayStatics.ApplyDamage` _array_element (`self.BR_MagicDMG`))
        (set `self.CheckHit` true)))))

(fn `UserConstructionScript`)