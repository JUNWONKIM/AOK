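; Short-lived boss attack actor (third attack) that plays a thunder sound, damages the player in its hitbox, and destroys itself after 0.7 seconds.
; Tick plays the sound once and schedules a flipbook swap for 0.7 seconds later, followed by an empty frame check.
; Tick also runs HitCheck behind a half-second Delay, applying BossATK3DMG to an overlapping BP_MainPlayer, with CheckHit limiting it to one hit.
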(event `self.ReceiveBeginPlay`
  (`KismetSystemLibrary.Delay` 0.7)
  (`self.K2_DestroyActor`))

(event `self.ReceiveTick`
  (params (DeltaSeconds :type "Float (single-precision)"))
  (`|ExecutionSequence`
    (:`then_0`
      (`/Engine/EditorBlueprintResources/StandardMacros.DoOnce` false
        (:`Completed`
          (`GameplayStatics.PlaySound2D` "/Game/Asset/Sound/Boss_Thunder.Boss_Thunder" 1.0 1.0 0.0 "/Game/Blueprint/BP_SoundConcurrency.BP_SoundConcurrency" null)
          (`KismetSystemLibrary.Delay` 0.7)
          (`PaperFlipbookComponent.SetFlipbook` (`self.Sprite`) "/Game/Asset/Boss/BossEffect/Boss_Atk4.Boss_Atk4")
          (if (== (`PaperFlipbookComponent.GetPlaybackPositionInFrames` (`self.Sprite`)) 7)
            _))))
    (:`then_1`
      (`KismetSystemLibrary.Delay` 0.5)
      (`self.HitCheck`))))

(fn `HitCheck`
  (for _array_element (`PrimitiveComponent.GetOverlappingActors` (`self.HitBox`) "/Game/Blueprint/BP_MainPlayer.BP_MainPlayer_C")
    (if (!= _array_element self)
      (if (not (`self.CheckHit`))
        (`GameplayStatics.ApplyDamage` _array_element (`self.Boss_ATK3_DMG`))
        (set `self.CheckHit` true)))))

(fn `UserConstructionScript`)