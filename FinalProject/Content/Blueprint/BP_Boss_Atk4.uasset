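; BP_Boss_Atk4 is a short-lived Paper2D boss magic attack that moves along negative X and damages the player.
; Tick applies movement input every frame and, through a DoOnce, waits half a second before swapping the flipbook, playing the magic sound and running HitCheck.
; HitCheck applies BRMagicDMG once to player actors overlapping the HitBox.
; The actor destroys itself one second after BeginPlay.
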(event `self.ReceiveBeginPlay`
  (`KismetSystemLibrary.Delay` 1.0)
  (`self.K2_DestroyActor`))

(event `self.ReceiveTick`
  (params (DeltaSeconds :type "Float (single-precision)"))
  (`|ExecutionSequence`
    (:`then_0`
      (`/Engine/EditorBlueprintResources/StandardMacros.DoOnce` false
        (:`Completed`
          (`KismetSystemLibrary.Delay` 0.5)
          (`PaperFlipbookComponent.SetFlipbook` (`self.Sprite`) "/Game/Asset/Boss/BossEffect/Dark_VFX_1/Separeted_frames/Boss_Atk1.Boss_Atk1")
          (`GameplayStatics.PlaySound2D` "/Game/Asset/Sound/BR_Magic.BR_Magic" 1.5 1.0 0.0 "/Game/Blueprint/BP_SoundConcurrency.BP_SoundConcurrency" null)
          (`self.HitCheck`))))
    (:`then_1`
      (`self.AddMovementInput` (-10.0 0.0 0.0) DeltaSeconds))))

(event `InputAxis|MoveRight`
  (params (AxisValue :type "Float (single-precision)")))

(fn `HitCheck`
  (for _array_element (`PrimitiveComponent.GetOverlappingActors` (`self.HitBox`) "/Game/Blueprint/BP_MainPlayer.BP_MainPlayer_C")
    (if (!= _array_element self)
      (`GameplayStatics.ApplyDamage` _array_element (`self.BR_MagicDMG`)))))

(fn `UserConstructionScript`)