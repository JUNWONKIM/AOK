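; Game mode that runs a rhythm-style countdown battle, creating the HUD widget and keeping shared state in BP_PlayerData.
; A looping timer ticks player and enemy counters while an enemy exists, with drum sounds marking the player count.
; Tick spawns, through a delay, a random enemy when none is active, or the boss once PDBossCount reaches zero.
; Tick also flags a critical attack at combo two and resets the combo at three.
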(event `self.ReceiveBeginPlay`
  (`|ExecutionSequence`
    (:`then_1`
      (bind _returnvalue (`|CreateWidget` "/Game/Blueprint/BP_Widget.BP_Widget_C"))
      (`UserWidget.AddToViewport` _returnvalue 0))
    (:`then_5`
      (bind _asbp_player_data (cast `/Game/Blueprint/BP_PlayerData` (`GameplayStatics.GetPlayerState` 0)))
      (set `self.As BP Player Data` _asbp_player_data))
    (:`then_7`
      ;[1 1 1] CountDown
      (`KismetSystemLibrary.Delay` 3.0)
      (`KismetSystemLibrary.K2_SetTimerDelegate` (delegate `PlayerATKCount`) 0.4 true))))

(event `PlayerATKCount`
  (bind _as_bp_player_data (`self.As BP Player Data`))
  (bind _as_bp_player_data_2 (`self.As BP Player Data`))
  ;[1 1 1] CountDown
  (if (`/Game/Blueprint/BP_PlayerData.PD_IsEnemySpawn` (`self.As BP Player Data`))
    (`|ExecutionSequence`
      (:`then_0`
        (if (!= (`/Game/Blueprint/BP_PlayerData.PD_PlayerCount` (`self.As BP Player Data`)) 0)
          (set `/Game/Blueprint/BP_PlayerData.PD_PlayerCount` (- (`/Game/Blueprint/BP_PlayerData.PD_PlayerCount` (`self.As BP Player Data`)) 1) (`self.As BP Player Data`))
          (if (!= (`/Game/Blueprint/BP_PlayerData.PD_PlayerCount` (`self.As BP Player Data`)) 0)
            (`GameplayStatics.SpawnSound2D` "/Game/Asset/Sound/Drum_low_40.Drum_low_40" 1.5 1.0 0.0 "/Game/Blueprint/BP_SoundConcurrency.BP_SoundConcurrency")
            (else
              (`GameplayStatics.SpawnSound2D` "/Game/Asset/Sound/Drum_hi_05.Drum_hi_05" 1.5 1.0 0.0 "/Game/Blueprint/BP_SoundConcurrency.BP_SoundConcurrency")))
          (else
            (set `/Game/Blueprint/BP_PlayerData.PD_PlayerCount` (+ (`KismetMathLibrary.RandomInteger` 8) 2) (`self.As BP Player Data`))
            (`GameplayStatics.SpawnSound2D` "/Game/Asset/Sound/Drum_low_40.Drum_low_40" 1.5 1.0 0.0 "/Game/Blueprint/BP_SoundConcurrency.BP_SoundConcurrency"))))
      (:`then_1`
        (if (!= (`/Game/Blueprint/BP_PlayerData.PD_EnemyCount` (`self.As BP Player Data`)) 0)
          (set `/Game/Blueprint/BP_PlayerData.PD_EnemyCount` (- (`/Game/Blueprint/BP_PlayerData.PD_EnemyCount` (`self.As BP Player Data`)) 1) (`self.As BP Player Data`))
          (else
            (set `/Game/Blueprint/BP_PlayerData.PD_EnemyCount` (`/Game/Blueprint/BP_PlayerData.PD_SetEnemyCount` _as_bp_player_data_2) _as_bp_player_data_2)))))
    (else
      (set `/Game/Blueprint/BP_PlayerData.PD_PlayerCount` 10 _as_bp_player_data)
      (set `/Game/Blueprint/BP_PlayerData.PD_EnemyCount` 5 _as_bp_player_data))))

(event `Spawn Enemy`
  ;[1 1 1] Spawn Enemy
  (if (`/Game/Blueprint/BP_PlayerData.PD_IsEnemySpawn` (`self.As BP Player Data`))
    _
    (elif (!= (`/Game/Blueprint/BP_PlayerData.PD_BossCount` (`self.As BP Player Data`)) 0)
      (switch `int` (`KismetMathLibrary.RandomInteger` 5)
        (:`0`
          (`|SpawnActorFromClass` "/Game/Blueprint/BP_NightBorne.BP_NightBorne_C" (`KismetMathLibrary.MakeTransform` (530.0 0.0 -300.0)) "Undefined" "OverrideRootScale" null null)
          (set `/Game/Blueprint/BP_PlayerData.PD_IsEnemySpawn` true (`self.As BP Player Data`)))
        (:`1`
          (`|SpawnActorFromClass` "/Game/Blueprint/BP_Bringer.BP_Bringer_C" (`KismetMathLibrary.MakeTransform` (530.0 0.0 -300.0)) "Undefined" "OverrideRootScale" null null)
          (set `/Game/Blueprint/BP_PlayerData.PD_IsEnemySpawn` true (`self.As BP Player Data`)))
        (:`2`
          (`|SpawnActorFromClass` "/Game/Blueprint/BP_Wizard.BP_Wizard_C" (`KismetMathLibrary.MakeTransform` (530.0 0.0 -300.0)) "Undefined" "OverrideRootScale" null null)
          (set `/Game/Blueprint/BP_PlayerData.PD_IsEnemySpawn` true (`self.As BP Player Data`))))
      (else
        (`|SpawnActorFromClass` "/Game/Blueprint/BP_Boss.BP_Boss_C" (`KismetMathLibrary.MakeTransform` (510.0 0.0 -300.0)) "Undefined" "OverrideRootScale" null null)
        (set `/Game/Blueprint/BP_PlayerData.PD_IsEnemySpawn` true (`self.As BP Player Data`))))))

(event `self.ReceiveTick`
  (params (DeltaSeconds :type "Float (single-precision)"))
  (bind _as_bp_player_data (`self.As BP Player Data`))
  (bind _as_bp_player_data_2 (`self.As BP Player Data`))
  (`|ExecutionSequence`
    (:`then_0`
      (`KismetSystemLibrary.Delay` 1.0)
      (`self.Spawn Enemy`))
    (:`then_3`
      (if (== (`/Game/Blueprint/BP_PlayerData.PD_PlayerComboCount` _as_bp_player_data) 2)
        (set `/Game/Blueprint/BP_PlayerData.PD_CRTAtk` true _as_bp_player_data)
        (else
          (set `/Game/Blueprint/BP_PlayerData.PD_CRTAtk` false _as_bp_player_data))))
    (:`then_5`
      (if (== (`/Game/Blueprint/BP_PlayerData.PD_PlayerComboCount` _as_bp_player_data_2) 3)
        (set `/Game/Blueprint/BP_PlayerData.PD_PlayerComboCount` 0 _as_bp_player_data_2)))))

(fn `UserConstructionScript`)