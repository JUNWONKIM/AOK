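; BP_NightBorne is a Paper2D boss enemy that attacks the player and updates shared BP_PlayerData state.
; Tick starts an attack when the enemy count reaches zero, then a DoOnce-gated flipbook frame triggers sound and hitbox overlap damage.
; Finished animations return to looping idle and reset the attack.
; Incoming damage raises player combo and plays hit or death animations, with death updating boss count, score and spawn state before destruction.
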(event `self.ReceiveBeginPlay`
  ;[0.7312 0.8408 1] NB_Count
  (`|ExecutionSequence`
    (:`then_0`
      (`PaperFlipbookComponent.SetFlipbook` (`self.Sprite`) "/Game/Asset/NightBorne/Night_Spawn.Night_Spawn")
      (`PaperFlipbookComponent.SetLooping` (`self.Sprite`) false))
    (:`then_3`
      (bind _asbp_player_data (cast `/Game/Blueprint/BP_PlayerData` (`GameplayStatics.GetPlayerState` 0)))
      (bind _output_get (set `self.As BP Player Data` _asbp_player_data))
      (set `/Game/Blueprint/BP_PlayerData.PD_SetEnemyCount` 7 _output_get))))

(event `Enemy Atk`
  ;[1 0.7554 0.5051] NB_Attack
  (if (== (`/Game/Blueprint/BP_PlayerData.PD_EnemyCount` (`self.As BP Player Data`)) 0)
    (if (`self.NB_TakeHit`)
      _
      (elif (not (`self.NB_Die`))
        (`PaperFlipbookComponent.SetFlipbook` (`self.Sprite`) "/Game/Asset/NightBorne/Night_Atk.Night_Atk")
        (set `/Game/Blueprint/BP_PlayerData.PD_CanBlockATK` true (`self.As BP Player Data`))
        (`PaperFlipbookComponent.SetLooping` (`self.Sprite`) false)
        (set `/Game/Blueprint/BP_PlayerData.PD_IsEnemyAttack` true (`self.As BP Player Data`))))))

(event `self.Sprite.OnFinishedPlaying`
  ;[0.4018 0.6503 1] NB_Idle
  (if (not (`self.NB_Die`))
    (`PaperFlipbookComponent.SetFlipbook` (`self.Sprite`) "/Game/Asset/NightBorne/Night_Idle.Night_Idle")
    (`self.Looping`)
    (set `/Game/Blueprint/BP_PlayerData.PD_IsEnemyAttack` false (`self.As BP Player Data`))
    (set `self.NB_TakeHit` false)
    (`self.ResetAttack`)
    (`SceneComponent.SetHiddenInGame` (`self.HitBox`) true false)))

(event `self.ReceiveTick`
  (params (DeltaSeconds :type "Float (single-precision)"))
  ;[1 0.9671 0.3297] Event Tick
  (`|ExecutionSequence`
    (:`then_2`
      (`self.Enemy Atk`))
    (:`then_4`
      (if (`/Game/Blueprint/BP_PlayerData.PD_IsEnemyAttack` (`self.As BP Player Data`))
        (if (== (`PaperFlipbookComponent.GetPlaybackPositionInFrames` (`self.Sprite`)) 7)
          (`/Engine/EditorBlueprintResources/StandardMacros.DoOnce` false :!label _label
            (:`Completed`
              (`GameplayStatics.PlaySound2D` "/Game/Asset/Sound/NB_Attack.NB_Attack" 1.0 1.0 0.0 "/Game/Blueprint/BP_SoundConcurrency.BP_SoundConcurrency" null)
              (`self.HitCheck`)
              (`SceneComponent.SetHiddenInGame` (`self.HitBox`) false false)))
          (else
            (`SceneComponent.SetHiddenInGame` (`self.HitBox`) true false)))))))

(event `ResetAttack`
  ;[1 0.9671 0.3297] Event Tick
  (goto _label :!via `Reset`))

(event `self.ReceiveAnyDamage`
  (params (Damage :type "Float (single-precision)") (DamageType :type "DamageType Object Reference") (InstigatedBy :type "Controller Object Reference") (DamageCauser :type "Actor Object Reference"))
  (bind _as_bp_player_data (`self.As BP Player Data`))
  (bind _nb_hp (`self.NB_HP`))
  (bind _as_bp_player_data_2 (`self.As BP Player Data`))
  (bind _as_bp_player_data_3 (`self.As BP Player Data`))
  ;[0.4464 0.3844 1] Get Damage
  (set `self.NB_HP` (- _nb_hp Damage))
  (if (<= _nb_hp 0.0)
    (set `self.NB_Die` true)
    (`GameplayStatics.PlaySound2D` "/Game/Asset/Sound/NB_Die.NB_Die" 0.5 1.0 0.0 "/Game/Blueprint/BP_SoundConcurrency.BP_SoundConcurrency" null)
    (`PaperFlipbookComponent.SetFlipbook` (`self.Sprite`) "/Game/Asset/NightBorne/Night_Die.Night_Die")
    (`PaperFlipbookComponent.SetLooping` (`self.Sprite`) false)
    (`|ExecutionSequence`
      (:`then_0`
        (`KismetSystemLibrary.Delay` 1.0)
        (set `/Game/Blueprint/BP_PlayerData.PD_IsEnemySpawn` false (`self.As BP Player Data`))
        (set `/Game/Blueprint/BP_PlayerData.PD_BossCount` (- (`/Game/Blueprint/BP_PlayerData.PD_BossCount` _as_bp_player_data_3) 1) _as_bp_player_data_3)
        (set `/Game/Blueprint/BP_PlayerData.PD_Score` (+ (`/Game/Blueprint/BP_PlayerData.PD_Score` _as_bp_player_data_2) 1) _as_bp_player_data_2)
        (`self.K2_DestroyActor`))
      (:`then_1`
        (set `/Game/Blueprint/BP_PlayerData.PD_PlayerComboCount` (+ (`/Game/Blueprint/BP_PlayerData.PD_PlayerComboCount` _as_bp_player_data) 1) _as_bp_player_data :!label _label_2)))
    (else
      (set `self.NB_TakeHit` true)
      (`PaperFlipbookComponent.SetFlipbook` (`self.Sprite`) "/Game/Asset/NightBorne/Night_TakeHit.Night_TakeHit")
      (`PaperFlipbookComponent.SetLooping` (`self.Sprite`) false)
      (goto _label_2))))

(fn `HitCheck`
  (for _array_element (`PrimitiveComponent.GetOverlappingActors` (`self.HitBox`) "/Game/Blueprint/BP_MainPlayer.BP_MainPlayer_C")
    (if (!= _array_element self)
      (if (not (`self.NB_Die`))
        (`GameplayStatics.ApplyDamage` _array_element (`self.NB_Damage`))))))

(fn `Looping`
  (`PaperFlipbookComponent.SetLooping` (`self.Sprite`) true)
  (if (not (`PaperFlipbookComponent.IsPlaying` (`self.Sprite`)))
    (`PaperFlipbookComponent.Play` (`self.Sprite`))))

(fn `UserConstructionScript`)