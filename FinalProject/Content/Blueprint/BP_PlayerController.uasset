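; Player controller that runs a random drum-beat countdown to open timed attack windows for the player.
; On BeginPlay it caches BP_PlayerData from the PlayerState and starts a looping half-second timer.
; Each beat decrements the count with a low drum, plays a high drum at zero, then rerolls a random count on the following beat.
; Tick sets the player data's attack flag true only while the count is zero.
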(event `self.ReceiveBeginPlay`
  (`|ExecutionSequence`
    (:`then_0`
      (bind _asbp_player_data (cast `/Game/Blueprint/BP_PlayerData` (`GameplayStatics.GetPlayerState` 0)))
      (set `self.As BP Player Data` _asbp_player_data))
    (:`then_3`
      (`KismetSystemLibrary.K2_SetTimerDelegate` (delegate `PlayerATKCount`) 0.5 true))))

(event `PlayerATKCount`
  (if (!= (`/Game/Blueprint/BP_PlayerData.PD_PlayerCount` (`self.As BP Player Data`)) 0)
    (set `/Game/Blueprint/BP_PlayerData.PD_PlayerCount` (- (`/Game/Blueprint/BP_PlayerData.PD_PlayerCount` (`self.As BP Player Data`)) 1) (`self.As BP Player Data`))
    (if (!= (`/Game/Blueprint/BP_PlayerData.PD_PlayerCount` (`self.As BP Player Data`)) 0)
      (`GameplayStatics.PlaySound2D` "/Game/Asset/Sound/Drum_low_40.Drum_low_40" 1.0 1.0 0.0 null null)
      (else
        (`GameplayStatics.PlaySound2D` "/Game/Asset/Sound/Drum_hi_05.Drum_hi_05" 1.0 1.0 0.0 null null)))
    (else
      (set `/Game/Blueprint/BP_PlayerData.PD_PlayerCount` (+ (`KismetMathLibrary.RandomInteger` 8) 2) (`self.As BP Player Data`))
      (`GameplayStatics.PlaySound2D` "/Game/Asset/Sound/Drum_low_40.Drum_low_40" 1.0 1.0 0.0 null null))))

(event `CanATK`
  (if (< (`/Game/Blueprint/BP_PlayerData.PD_PlayerCount` (`self.As BP Player Data`)) 1)
    (set `/Game/Blueprint/BP_PlayerData.PD_CanAttack` true (`self.As BP Player Data`))
    (else
      (set `/Game/Blueprint/BP_PlayerData.PD_CanAttack` false (`self.As BP Player Data`)))))

(event `self.ReceiveTick`
  (params (DeltaSeconds :type "Float (single-precision)"))
  (`self.CanATK`))

(fn `UserConstructionScript`)