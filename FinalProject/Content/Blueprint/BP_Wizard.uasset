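; BP_Wizard is a flipbook-animated enemy that spawns, attacks the player, takes damage and dies.
; Each tick it starts an attack when the enemy count in BP_PlayerData reaches zero, sharing attack, block and spawn flags there.
; Two frame-timed DoOnce gates deal damage through HitBox overlaps; finishing an animation returns it to idle and re-arms them.
; Lethal damage plays death, clears the spawn flag and destroys it.
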(event `self.ReceiveBeginPlay`
  ;[0.7312 0.8408 1] NB_Count
  (`|ExecutionSequence`
    (:`then_0`
      (`PaperFlipbookComponent.SetFlipbook` (`self.Sprite`) "/Game/Asset/EVil_Wizard_2/Sprites/Wizard_Spawn.Wizard_Spawn")
      (`PaperFlipbookComponent.SetLooping` (`self.Sprite`) false))
    (:`then_3`
      (bind _asbp_player_data (cast `/Game/Blueprint/BP_PlayerData` (`GameplayStatics.GetPlayerState` 0)))
      (bind _output_get (set `self.As BP Player Data` _asbp_player_data))
      (set `/Game/Blueprint/BP_PlayerData.PD_SetEnemyCount` 6 _output_get))))

(event `Enemy Atk`
  ;[1 0.7554 0.5051] NB_Attack
  (if (== (`/Game/Blueprint/BP_PlayerData.PD_EnemyCount` (`self.As BP Player Data`)) 0)
    (if (`self.WZ_TakeHit`)
      _
      (elif (not (`self.WZ_Die`))
        (`PaperFlipbookComponent.SetFlipbook` (`self.Sprite`) "/Game/Asset/EVil_Wizard_2/Sprites/Wizard_ATK.Wizard_ATK")
        (set `/Game/Blueprint/BP_PlayerData.PD_CanBlockATK` true (`self.As BP Player Data`))
        (`PaperFlipbookComponent.SetLooping` (`self.Sprite`) false)
        (set `/Game/Blueprint/BP_PlayerData.PD_IsEnemyAttack` true (`self.As BP Player Data`))))))

(event `self.Sprite.OnFinishedPlaying`
  ;[0.4018 0.6503 1] NB_Idle
  (if (not (`self.WZ_Die`))
    (`PaperFlipbookComponent.SetFlipbook` (`self.Sprite`) "/Game/Asset/EVil_Wizard_2/Sprites/Wizard_Idle.Wizard_Idle")
    (`self.Looping`)
    (set `/Game/Blueprint/BP_PlayerData.PD_IsEnemyAttack` false (`self.As BP Player Data`))
    (set `self.WZ_TakeHit` false)
    (`self.ResetAttack`)
    (`SceneComponent.SetHiddenInGame` (`self.HitBox`) true false)))

(event `self.ReceiveTick`
  (params (DeltaSeconds :type "Float (single-precision)"))
  ;[1 0.9671 0.3297] Event Tick
  (`|ExecutionSequence`
    (:`then_2`
      (`self.Enemy Atk`))
    (:`then_4`
      (if (`/Game/Blueprint/BP_PlayerData.PD_IsEnemyAttack` (`self.As BP Player Data`))
        (`|ExecutionSequence`
          (:`then_0`
            (if (== (`PaperFlipbookComponent.GetPlaybackPositionInFrames` (`self.Sprite`)) 3)
              (`/Engine/EditorBlueprintResources/StandardMacros.DoOnce` false :!label _label
                (:`Completed`
                  (`GameplayStatics.PlaySound2D` "/Game/Asset/Sound/NB_Attack.NB_Attack" 1.0 1.0 0.0 "/Game/Blueprint/BP_SoundConcurrency.BP_SoundConcurrency" null)
                  (`self.HitCheck`)
                  (`SceneComponent.SetHiddenInGame` (`self.HitBox`) true false)))))
          (:`then_1`
            (if (== (`PaperFlipbookComponent.GetPlaybackPositionInFrames` (`self.Sprite`)) 12)
              (`/Engine/EditorBlueprintResources/StandardMacros.DoOnce` false :!label _label_2
                (:`Completed`
                  (`GameplayStatics.PlaySound2D` "/Game/Asset/Sound/NB_Attack.NB_Attack" 1.0 1.0 0.0 "/Game/Blueprint/BP_SoundConcurrency.BP_SoundConcurrency" null)
                  (`self.HitCheck`)
                  (`SceneComponent.SetHiddenInGame` (`self.HitBox`) true false))))))))))

(event `ResetAttack`
  ;[1 0.9671 0.3297] Event Tick
  (`|ExecutionSequence`
    (:`then_0`
      (goto _label :!via `Reset`))
    (:`then_1`
      (goto _label_2 :!via `Reset`))))

(event `self.ReceiveAnyDamage`
  (params (Damage :type "Float (single-precision)") (DamageType :type "DamageType Object Reference") (InstigatedBy :type "Controller Object Reference") (DamageCauser :type "Actor Object Reference"))
  (bind _wz_hp (`self.WZ_HP`))
  ;[0.4464 0.3844 1] Get Damage
  (set `self.WZ_HP` (- _wz_hp Damage))
  (if (<= _wz_hp 0.0)
    (set `self.WZ_Die` true)
    (`GameplayStatics.PlaySound2D` "/Game/Asset/Sound/NB_Die.NB_Die" 0.5 1.0 0.0 "/Game/Blueprint/BP_SoundConcurrency.BP_SoundConcurrency" null)
    (`PaperFlipbookComponent.SetFlipbook` (`self.Sprite`) "/Game/Asset/EVil_Wizard_2/Sprites/Wizard_Death.Wizard_Death")
    (`PaperFlipbookComponent.SetLooping` (`self.Sprite`) false)
    (`KismetSystemLibrary.Delay` 1.0)
    (set `/Game/Blueprint/BP_PlayerData.PD_IsEnemySpawn` false (`self.As BP Player Data`))
    (`self.K2_DestroyActor`)
    (else
      (set `self.WZ_TakeHit` true)
      (`PaperFlipbookComponent.SetFlipbook` (`self.Sprite`) "/Game/Asset/EVil_Wizard_2/Sprites/Wizard_TakeHit.Wizard_TakeHit")
      (`PaperFlipbookComponent.SetLooping` (`self.Sprite`) false))))

(fn `HitCheck`
  (for _array_element (`PrimitiveComponent.GetOverlappingActors` (`self.HitBox`) "/Game/Blueprint/BP_MainPlayer.BP_MainPlayer_C")
    (if (!= _array_element self)
      (if (not (`self.WZ_Die`))
        (`GameplayStatics.ApplyDamage` _array_element (`self.WZ_Damage`))))))

(fn `Looping`
  (`PaperFlipbookComponent.SetLooping` (`self.Sprite`) true)
  (if (not (`PaperFlipbookComponent.IsPlaying` (`self.Sprite`)))
    (`PaperFlipbookComponent.Play` (`self.Sprite`))))

(fn `UserConstructionScript`)